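; Cube actor that changes its mesh material when used, either cycling through a material array or copying the cube to its right.
; BeginPlay advances the cycle once; OnUse calls ChangeMaterial or, when CopyRight is set, CopyRightMaterial, then prints the material name.
; The copy mode runs a debug-drawn Visibility line trace along the right vector and takes the material from the Cube_BP it hits.
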(event EventBeginPlay
  (CallFunction|ChangeMaterial) ; En caso de probar el que cambie de color en ciclo hay que conectarlo para que empiece en el 1
)

(fn ConstructionScript
  (|CallParentFunction))

(fn ChangeMaterial
  ;[1 1 1] Change Material Cycle
  (bind _result (Math|Integer|IncrementInt (Variables|Default|GetCurrentIdMaterial))
    (:%20%20
      (if (<= _result (- (Utilities|Array|Length (Variables|Default|GetMaterial)) 1))
        _
        (else
          (Variables|Default|SetCurrentIdMaterial 0)))
      (Rendering|Material|SetMaterial (Variables|Default|GetCubeMesh) 0 (Utilities|Array|Get(acopy) (Variables|Default|GetMaterial) (Variables|Default|GetCurrentIdMaterial))))))

(fn OnUse
  (if (Variables|Default|GetbCopyRight)
    (CallFunction|CopyRightMaterial)
    (else
      (CallFunction|ChangeMaterial)))
  (CallFunction|PrintNameMaterial))

(fn PrintNameMaterial
  ;[1 1 1] Print Name Material
  (Development|PrintString (Utilities|GetDisplayName (Rendering|Material|GetMaterial (Variables|Default|GetCubeMesh) 0))))

(fn GetMaterial
  (return (Rendering|Material|GetMaterial (Variables|Default|GetCubeMesh) 0)))

(fn CopyRightMaterial
  (bind (_outhit _returnvalue) (Collision|LineTraceByChannel (Utilities|GetLocation 4e+01) (Utilities|GetLocation 4e+02) "TraceTypeQuery1" false 0 "ForDuration" true "(R=1.000000,G=0.000000,B=0.000000,A=1.000000)" "(R=0.000000,G=1.000000,B=0.000000,A=1.000000)" 3.0))
  (if _returnvalue
    (bind _ascube_bp (Utilities|Casting|CastToCube_BP (.hitactor _outhit)))
    (bind _material (CallFunction|GetMaterial _ascube_bp))
    (Rendering|Material|SetMaterial (Variables|Default|GetCubeMesh) 0 _material)))
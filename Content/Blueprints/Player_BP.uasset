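; Player Blueprint that lets the player use items in front of them.
; Pressing Use fires a debug-drawn Visibility line trace along the control rotation and calls OnUse on any ItemClass_BP it hits.
; GetLocation supplies both trace endpoints, using a math expression to project a given distance from the actor's location.
; An older fixed-distance End function remains but is unused.
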(event Input|ActionEvents|InputActionUse
  (params (Key :type Key%20Structure :default "None"))
  (:Pressed
    (bind (_outhit _returnvalue) (Collision|LineTraceByChannel (Utilities|GetLocation 4e+01) (Utilities|GetLocation 4e+02) "TraceTypeQuery1" false 0 "ForDuration"))
    (if _returnvalue
      (bind _asitem_class_bp (Utilities|Casting|CastToItemClass_BP (.hitactor _outhit)))
      (Default|OnUse _asitem_class_bp))))

(fn ConstructionScript)
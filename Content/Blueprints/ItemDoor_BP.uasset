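; Usable door item that swings open or closed each time it is used.
; OnUse flips IsOpen and calls ChangeDoorState, which plays the Door_TL timeline from the start to open or reverses it from the end to close.
; The timeline track drives the relative yaw of the Scene component.
; The construction script only calls its parent, leaving a disconnected node that would size the Box to the mesh bounds.
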(event Custom|ChangeDoorState
  (if (Variables|Default|GetbIsOpen)
    (bind _track (Timeline|Door_TL PlayFromStart)
      (:Update
        (Transformation|SetRelativeRotation (Variables|Default|GetScene) (Math|Rotator|MakeRotator 0.0 0.0 _track) false false)))
    (else
      (Timeline|Door_TL ReverseFromEnd))))

(fn ConstructionScript
  (|CallParentFunction))

(fn OnUse
  (Variables|Default|SetbIsOpen (not (Variables|Default|GetbIsOpen)))
  (CallFunction|ChangeDoorState))